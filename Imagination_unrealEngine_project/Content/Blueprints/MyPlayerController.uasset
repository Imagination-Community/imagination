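; Player controller Blueprint that routes Enhanced Input actions to player gameplay functions.
; On BeginPlay it adds the player input mapping context to the local player subsystem.
; Input events forward movement, camera and rotation values, and trigger jumping, grapnel enable and disable, item take or place, and pawn upgrade.
; The called functions are defined outside the graphs shown; Tick and the construction script are empty.
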(event Input|EnhancedActionEvents|EnhancedInputActionPlayerMove
  (params (ActionValue :type Vector%202D%20Structure) (ElapsedSeconds :type Float%20%28double-precision%29) (TriggeredSeconds :type Float%20%28double-precision%29) (InputAction :type Input%20Action%20Object%20Reference :default "/Game/Input/PlayerMove.PlayerMove"))
  (:Triggered
    (Class|MyPlayerController|Move ActionValue)))

(event Input|EnhancedActionEvents|EnhancedInputActionCameraMove
  (params (ActionValue :type Vector%202D%20Structure) (ElapsedSeconds :type Float%20%28double-precision%29) (TriggeredSeconds :type Float%20%28double-precision%29) (InputAction :type Input%20Action%20Object%20Reference :default "/Game/Input/CameraMove.CameraMove"))
  (:Triggered
    (Class|MyPlayerController|RotateCamera ActionValue)))

(event Input|EnhancedActionEvents|EnhancedInputActionPlayerRotate
  (params (ActionValue :type Float%20%28double-precision%29) (ElapsedSeconds :type Float%20%28double-precision%29) (TriggeredSeconds :type Float%20%28double-precision%29) (InputAction :type Input%20Action%20Object%20Reference :default "/Game/Input/PlayerRotate.PlayerRotate"))
  (:Triggered
    (Class|MyPlayerController|Rotate ActionValue)))

(event Input|EnhancedActionEvents|EnhancedInputActionPlayerGrappin
  (params (ActionValue :type Boolean) (ElapsedSeconds :type Float%20%28double-precision%29) (TriggeredSeconds :type Float%20%28double-precision%29) (InputAction :type Input%20Action%20Object%20Reference :default "/Game/Input/PlayerGrappin.PlayerGrappin"))
  (:Started
    (Class|MyPlayerController|EnableGrapnel)))

(event Input|EnhancedActionEvents|EnhancedInputActionDisableGrappin
  (params (ActionValue :type Boolean) (ElapsedSeconds :type Float%20%28double-precision%29) (TriggeredSeconds :type Float%20%28double-precision%29) (InputAction :type Input%20Action%20Object%20Reference :default "/Game/Input/DisableGrappin.DisableGrappin"))
  (:Started
    (Class|MyPlayerController|DisableGrapnel)))

(event Input|EnhancedActionEvents|EnhancedInputActionPlayerJump
  (params (ActionValue :type Boolean) (ElapsedSeconds :type Float%20%28double-precision%29) (TriggeredSeconds :type Float%20%28double-precision%29) (InputAction :type Input%20Action%20Object%20Reference :default "/Game/Input/PlayerJump.PlayerJump"))
  (:Started
    (Class|MyPlayerController|Jump)))

(event Input|EnhancedActionEvents|EnhancedInputActionPlayerTakeOrPlaceItem
  (params (ActionValue :type Boolean) (ElapsedSeconds :type Float%20%28double-precision%29) (TriggeredSeconds :type Float%20%28double-precision%29) (InputAction :type Input%20Action%20Object%20Reference :default "/Game/Input/PlayerTakeOrPlaceItem.PlayerTakeOrPlaceItem"))
  (:Started
    (Class|MyPlayerController|TakeorPlaceItem)))

(event Input|EnhancedActionEvents|EnhancedInputActionPlayerUpgrade
  (params (ActionValue :type Boolean) (ElapsedSeconds :type Float%20%28double-precision%29) (TriggeredSeconds :type Float%20%28double-precision%29) (InputAction :type Input%20Action%20Object%20Reference :default "/Game/Input/PlayerUpgrade.PlayerUpgrade"))
  (:Started
    (Class|MyPlayerController|UpgradePawn)))

(event EventBeginPlay
  (Input|AddMappingContext (PlayerController|LocalPlayerSubsystems|GetEnhancedInputLocalPlayerSubsystem self) "/Game/Input/PlayerInputMappingContext.PlayerInputMappingContext" 0 "(bIgnoreAllPressedKeysUntilRelease=True,bForceImmediately=False)")
  (Variables|Default|SetAs%20Player%20Controller 0))

(event EventTick
  (params (DeltaSeconds :type Float%20%28single-precision%29)))

(fn ConstructionScript)